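; CPU opponent paddle that serves and returns physics balls, scaled by game difficulty.
; Game mode events spawn and launch a new ball, while a gated overlap returns balls with matching launcher and last-hit surface.
; Launches use SuggestProjectileVelocityCustomArc toward a random point in a difficulty-scaled destination box, with a timeline rotating the paddle mesh.
; Each tick the paddle follows the incoming ball or drifts home, clamped to a difficulty-scaled movement area.
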(event `self.ReceiveBeginPlay`
  ;[0.195 0.1697 0] Begin Play
  (bind _asbp_game_mode (cast `/Game/Blueprints/BP_GameMode` (`GameplayStatics.GetGameMode`)))
  (add `/Game/Blueprints/BP_GameMode.On Match Started` _asbp_game_mode (delegate `On Match Started`))
  (add `/Game/Blueprints/BP_GameMode.On Spawn New Ball Requested` _asbp_game_mode (delegate `On Spawn New Ball Requested`)))

(event `On Spawn New Ball Requested`
  ;[0.195 0.1697 0] Begin Play
  (`self.Spawn New Ball` :!label _label))

(event `On Match Started`
  ;[0.195 0.1697 0] Begin Play
  (goto _label))

(event `self.ReceiveTick`
  (params (DeltaSeconds :type "Float (single-precision)"))
  ;[0 0.03585 0.15] Tick
  (`self.Move Cpu Paddle` DeltaSeconds))

(event `self.Paddle_StaticMesh.OnComponentBeginOverlap`
  (params (OverlappedComponent :type "PrimitiveComponent Object Reference") (OtherActor :type "Actor Object Reference") (OtherComp :type "PrimitiveComponent Object Reference") (OtherBodyIndex :type Integer) (bFromSweep :type Boolean) (SweepResult :type "HitResult Structure (by ref)"))
  ;[0.1356 0.1946 0.4735] Begin Overlap
  (`/Engine/EditorBlueprintResources/StandardMacros.Gate` true :!label _label_2
    (:`Exit`
      (bind _asbp_physics_ball_actor (cast `/Game/Blueprints/BP_PhysicsBallActor` OtherActor))
      (`/Engine/EditorBlueprintResources/StandardMacros.DoOnce` false :!label _label_3
        (:`Completed`
          (if (and (`|EnumEquality` (`/Game/Blueprints/BP_PhysicsBallActor.Current Launcher` _asbp_physics_ball_actor) "NewEnumerator1") (`|EnumEquality` (`/Game/Blueprints/BP_PhysicsBallActor.Last Hit Surface` _asbp_physics_ball_actor) "NewEnumerator2"))
            (bind _return_vlaue (message `/Game/Blueprints/BP_GameModeInterface.Get Difficulty Level` (`GameplayStatics.GetGameMode`)))
            (`self.On Ball Launch` _asbp_physics_ball_actor _return_vlaue)
            (`KismetSystemLibrary.Delay` 1.0)
            (goto _label_3 :!via `Reset`)
            (else
              (goto _label_3 :!via `Reset`))))))))

(event `Set Overlap Detection Active`
  (params (`Is Active ?` :type Boolean))
  ;[0.1356 0.1946 0.4735] Begin Overlap
  (if `Is Active ?`
    (goto _label_2 :!via `Open`)
    (else
      (goto _label_2 :!via `Close`))))

(event `Spawn New Ball`
  ;[0.175 0 0] Custom Events
  (`/Engine/EditorBlueprintResources/StandardMacros.DoOnce` false :!label _label_4
    (:`Completed`
      (`self.Set Overlap Detection Active` false)
      (`KismetSystemLibrary.Delay` 0.5)
      (bind _return_vlaue (message `/Game/Blueprints/BP_GameModeInterface.Get Difficulty Level` (`GameplayStatics.GetGameMode`)))
      (bind _returnvalue (`|SpawnActorFromClass` "/Game/Blueprints/BP_PhysicsBallActor.BP_PhysicsBallActor_C" (`KismetMathLibrary.MakeTransform` (`SceneComponent.K2_GetComponentLocation` (`self.BallSpawnPoint`)) (struct)) "Undefined" "OverrideRootScale" null false (select `/Game/Blueprints/Enum_DifficultyLevel` _return_vlaue :`NewEnumerator0` 350.0 :`NewEnumerator1` 700.0 :`NewEnumerator2` 4000.0 :!type "Float (single-precision)") null))
      (bind _return_value (message `/Game/Blueprints/BP_GameModeInterface.Set Ball Reference` (`GameplayStatics.GetGameMode`) _returnvalue))
      (`self.On Ball Launch` _return_value _return_vlaue)
      (`KismetSystemLibrary.Delay` 1.0)
      (`self.Set Overlap Detection Active` true)
      (goto _label_4 :!via `Reset`))))

(event `On Ball Launch`
  (params (`Current Ball` :type "/Game/Blueprints/BP_PhysicsBallActor Object Reference") (`Current Difficulty` :type "/Game/Blueprints/Enum_DifficultyLevel Enum" :default "NewEnumerator0"))
  (bind (_arc_param_min _arc_param_max) (`self.Get Arc Param Bounds Based On Difficulty` `Current Difficulty`))
  ;[0.175 0 0] Custom Events
  (`/Engine/EditorBlueprintResources/StandardMacros.IsValid` `Current Ball`
    (:`Is Valid`
      (bind _launchvelocity (`self.Get Random Launch Velocity` (`self.K2_GetActorLocation` `Current Ball`) (`self.Get Box Scale Ratio Based On Difficulty` `Current Difficulty`) _arc_param_min _arc_param_max))
      (`/Game/Blueprints/BP_PhysicsBallActor.Launch Ball` `Current Ball` "NewEnumerator0" _launchvelocity)
      (`self.Play Launch Animation` (`KismetMathLibrary.Normal` _launchvelocity)))))

(event `Play Launch Animation`
  (params (`Launch Direction` :type "Vector Structure"))
  ;[0.175 0 0] Custom Events
  (bind (_direction _lerpalpha) (`Timeline|Launch Animation Timeline` :!via `PlayFromStart`)
    (:`Update`
      (`SceneComponent.K2_SetWorldRotation` (`self.Paddle_StaticMesh`) (`KismetMathLibrary.RLerp` (struct :`Yaw` -180.0) (`KismetMathLibrary.Conv_VectorToRotator` `Launch Direction`) _lerpalpha true) false false))))

(fn `Get Arc Param Bounds Based On Difficulty`
  (params (`Current Difficulty` :type "/Game/Blueprints/Enum_DifficultyLevel Enum" :default "NewEnumerator0"))
  (returns (`Arc Param Min` :type "Float (double-precision)") (`Arc Param Max` :type "Float (double-precision)"))
  (return (select `/Game/Blueprints/Enum_DifficultyLevel` `Current Difficulty` :`NewEnumerator0` 0.5 :`NewEnumerator1` 0.4 :`NewEnumerator2` 0.6 :!type "Float (single-precision)") (select `/Game/Blueprints/Enum_DifficultyLevel` `Current Difficulty` :`NewEnumerator0` 0.5 :`NewEnumerator1` 0.6 :`NewEnumerator2` 0.75 :!type "Float (single-precision)")))

(fn `Get Box Scale Ratio Based On Difficulty`
  (params (`Current Difficulty` :type "/Game/Blueprints/Enum_DifficultyLevel Enum" :default "NewEnumerator0"))
  (returns (`Return value` :type "Float (double-precision)"))
  (return (select `/Game/Blueprints/Enum_DifficultyLevel` `Current Difficulty` :`NewEnumerator0` 0.5 :`NewEnumerator1` 0.75 :`NewEnumerator2` 1.0 :!type "Float (single-precision)")))

(fn `Get Random Launch Velocity`
  (params (StartPosition :type "Vector Structure") (`Destination Box Scale Ratio` :type "Float (double-precision)") (`Arc Param Min` :type "Float (double-precision)" :default 0.0) (`Arc Param Max` :type "Float (double-precision)" :default 1.0))
  (returns (LaunchVelocity :type "Vector Structure"))
  (bind (_origin _boxextent) (`KismetSystemLibrary.GetComponentBounds` (`self.Ball Destination Box`)))
  (bind (_outlaunchvelocity _returnvalue) (`GameplayStatics.SuggestProjectileVelocity_CustomArc` StartPosition (`KismetMathLibrary.RandomPointInBoundingBox` _origin (* _boxextent `Destination Box Scale Ratio`)) 0.0 (`KismetMathLibrary.RandomFloatInRange` `Arc Param Min` `Arc Param Max`)))
  (return (select `bool` _returnvalue :`false` (-500.0 0.0 0.0) :`true` _outlaunchvelocity)))

(fn `Move Cpu Paddle`
  (params (`Delta Time` :type "Float (double-precision)"))
  (locals (`Delta Seconds` :type "Float (double-precision)"))
  (bind _paddle_root (`self.Paddle_ROOT`))
  (bind _paddle_root_2 (`self.Paddle_ROOT`))
  (bind _paddle_root_3 (`self.Paddle_ROOT`))
  (bind _paddle_root_4 (`self.Paddle_ROOT`))
  (bind (_origin _boxextent) (`KismetSystemLibrary.GetComponentBounds` (`self.Paddle Movement Area`)))
  (bind _x (.x _origin))
  (bind _y (.y _origin))
  (bind _z (.z _origin))
  (set `local.Delta Seconds` `Delta Time`)
  (bind _return_vlaue (message `/Game/Blueprints/BP_GameModeInterface.Get Difficulty Level` (`GameplayStatics.GetGameMode`)))
  (`|ExecutionSequence`
    (:`then_0`
      (bind _returnvalue (message `/Game/Blueprints/BP_GameModeInterface.Get Current Ball` (`GameplayStatics.GetGameMode`)))
      (`/Engine/EditorBlueprintResources/StandardMacros.IsValid` _returnvalue
        (:`Is Valid`
          (if (`/Game/Blueprints/BP_PhysicsBallActor.Is Active Ball ?` _returnvalue)
            (if (> (.x (`self.GetVelocity` _returnvalue)) 0.0)
              (bind _last_hit_surface (`/Game/Blueprints/BP_PhysicsBallActor.Last Hit Surface` _returnvalue))
              (if (`|EnumEquality` _last_hit_surface "NewEnumerator3")
                (bind _returnvalue_2 (`self.K2_GetActorLocation` _returnvalue))
                (`SceneComponent.K2_SetWorldLocation` _paddle_root_2 (`KismetMathLibrary.VInterpTo_Constant` (`SceneComponent.K2_GetComponentLocation` _paddle_root_2) (`KismetMathLibrary.MakeVector` (.x (`SceneComponent.K2_GetComponentLocation` (`self.Dummy_ROOT`))) (.y _returnvalue_2) (.z (`SceneComponent.K2_GetComponentLocation` (`self.Dummy_ROOT`)))) (`local.Delta Seconds`) 500.0) false false)
                (elif (`|EnumEquality` _last_hit_surface "NewEnumerator2")
                  (`SceneComponent.K2_SetWorldLocation` _paddle_root_3 (`KismetMathLibrary.VInterpTo_Constant` (`SceneComponent.K2_GetComponentLocation` _paddle_root_3) _returnvalue_2 (`local.Delta Seconds`) 500.0) false false)))
              (else
                (`SceneComponent.K2_SetWorldLocation` _paddle_root (`KismetMathLibrary.VInterpTo_Constant` (`SceneComponent.K2_GetComponentLocation` _paddle_root) (`SceneComponent.K2_GetComponentLocation` (`self.Dummy_ROOT`)) (`local.Delta Seconds`) 500.0) false false :!label _label)))
            (else
              (goto _label))))
        (:`Is Not Valid`
          (goto _label))))
    (:`then_1`
      (bind _x_2 (.x (* _boxextent (`self.Get Box Scale Ratio Based On Difficulty` _return_vlaue))))
      (bind _y_2 (.y (* _boxextent (`self.Get Box Scale Ratio Based On Difficulty` _return_vlaue))))
      (bind _z_2 (.z (* _boxextent (`self.Get Box Scale Ratio Based On Difficulty` _return_vlaue))))
      (`SceneComponent.K2_SetWorldLocation` _paddle_root_4 (`KismetMathLibrary.MakeVector` (`KismetMathLibrary.FClamp` (.x (`SceneComponent.K2_GetComponentLocation` _paddle_root_4)) (- _x _x_2) (+ _x _x_2)) (`KismetMathLibrary.FClamp` (.y (`SceneComponent.K2_GetComponentLocation` _paddle_root_4)) (- _y _y_2) (+ _y _y_2)) (`KismetMathLibrary.FClamp` (.z (`SceneComponent.K2_GetComponentLocation` _paddle_root_4)) (- _z _z_2) (+ _z _z_2))) false false))))

(fn `UserConstructionScript`
  (bind _returnvalue (`SceneComponent.K2_GetComponentLocation` (`self.BallSpawnPoint`)))
  (bind _returnvalue_2 (- (`SceneComponent.K2_GetComponentLocation` (`self.Ball Destination Box`)) _returnvalue))
  (`SceneComponent.K2_SetRelativeTransform` (`self.Ball Destination Box`) (`self.Ball Destination Box Transform`) false false)
  (`SceneComponent.K2_SetRelativeTransform` (`self.Paddle Movement Area`) (`self.Paddle Movement Area Transform`) false false)
  (`SceneComponent.K2_SetWorldLocationAndRotation` (`self.Arrow`) _returnvalue (`KismetMathLibrary.Conv_VectorToRotator` _returnvalue_2) false false)
  (`SceneComponent.SetRelativeScale3D` (`self.Arrow`) (`KismetMathLibrary.MakeVector` (/ (`KismetMathLibrary.VSize` _returnvalue_2) 50.0) 1.0 1.0)))