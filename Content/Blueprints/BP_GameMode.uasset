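; Game mode for a Player 1 vs CPU ball game, owning the score, difficulty level and current ball reference.
; Game mode interface events update state and broadcast it through dispatchers for score, match, UI interaction and ball spawning.
; Each point either requests a new ball or ends the match once a side reaches seven with a two-point lead.
; UI interaction starts shortly after BeginPlay and at match end, and stops when a new match starts.
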(event `self.ReceiveBeginPlay`
  ;[0.19 0.1746 0] Begin Play
  (`KismetSystemLibrary.Delay` 0.5)
  (`self.On UI Interaction Started`))

(event `/Game/Blueprints/BP_GameModeInterface.Update Score`
  (params (Target :type "/Game/Blueprints/Enum_PlayerType Enum"))
  ;[0.08 0 0] GameMode Interface Events
  (`|ExecutionSequence`
    (:`then_0`
      (switch `/Game/Blueprints/Enum_PlayerType` Target
        (:`NewEnumerator0`
          (`/Engine/EditorBlueprintResources/StandardMacros.IncrementInt` (`self.Cpu Score`)))
        (:`NewEnumerator1`
          (`/Engine/EditorBlueprintResources/StandardMacros.IncrementInt` (`self.Player1 Score`)))))
    (:`then_1`
      (`self.On Score Updated` (`self.Cpu Score`) (`self.Player1 Score`)))
    (:`then_2`
      (if (and (>= (`KismetMathLibrary.Abs_Int` (- (`self.Player1 Score`) (`self.Cpu Score`))) 2) (or (>= (`self.Player1 Score`) 7) (>= (`self.Cpu Score`) 7)))
        (`self.On Match Ended` (select `bool` (> (`self.Player1 Score`) (`self.Cpu Score`)) :`false` "NewEnumerator0" :`true` "NewEnumerator1" :!type "/Game/Blueprints/Enum_PlayerType Enum"))
        (`self.On UI Interaction Started`)
        (else
          (`self.On Spawn New Ball Requested`))))))

(event `/Game/Blueprints/BP_GameModeInterface.Set Difficulty Level`
  (params (`New Difficulty` :type "/Game/Blueprints/Enum_DifficultyLevel Enum" :default "NewEnumerator0"))
  ;[0.08 0 0] GameMode Interface Events
  (set `self.Current Difficulty Level` `New Difficulty`))

(event `/Game/Blueprints/BP_GameModeInterface.Start New Match`
  ;[0.08 0 0] GameMode Interface Events
  (`self.On UI Interaction Ended`)
  (set `self.Player1 Score` 0)
  (set `self.Cpu Score` 0)
  (`self.On Match Started`)
  (`self.On Score Updated` 0))

(event `/Game/Blueprints/BP_GameModeInterface.Set UI Interaction Active`
  (params (`Is Active ?` :type Boolean))
  ;[0.08 0 0] GameMode Interface Events
  (if `Is Active ?`
    (`self.On UI Interaction Started`)
    (else
      (`self.On UI Interaction Ended`))))

(fn `Get Current Ball`
  (returns (ReturnValue :type "/Game/Blueprints/BP_PhysicsBallActor Object Reference"))
  (return (`self.Current Ball Reference`)))

(fn `Get Difficulty Level`
  (returns (`Return Vlaue` :type "/Game/Blueprints/Enum_DifficultyLevel Enum"))
  (return (`self.Current Difficulty Level`)))

(fn `Set Ball Reference`
  (params (`New Ball` :type "/Game/Blueprints/BP_PhysicsBallActor Object Reference"))
  (returns (`Return Value` :type "/Game/Blueprints/BP_PhysicsBallActor Object Reference"))
  (bind _output_get (set `self.Current Ball Reference` `New Ball`))
  (return _output_get))

(fn `UserConstructionScript`)