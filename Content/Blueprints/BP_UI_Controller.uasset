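; VR UI pointer that shows a laser and clicks widgets with the right motion controller trigger through a WidgetInteraction component.
; Game mode UI interaction started/ended events toggle hit testing and laser visibility, both off at start.
; A status macro gates Tick and input on hit testing, so active frames rescale the laser from hit data and the trigger simulates left mouse clicks.
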(event `self.ReceiveBeginPlay`
  ;[0.185 0.167 0] Begin Play
  (`self.Set Hit Testing Enabled` false)
  (bind _asbp_game_mode (cast `/Game/Blueprints/BP_GameMode` (`GameplayStatics.GetGameMode`)))
  (add `/Game/Blueprints/BP_GameMode.On UI Interaction Started` _asbp_game_mode (delegate `On UI Interaction Started`))
  (add `/Game/Blueprints/BP_GameMode.On UI Interaction Ended` _asbp_game_mode (delegate `On UI Interaction Ended`)))

(event `On UI Interaction Ended`
  ;[0.185 0.167 0] Begin Play
  (`self.Set Hit Testing Enabled` false))

(event `On UI Interaction Started`
  ;[0.185 0.167 0] Begin Play
  (`self.Set Hit Testing Enabled` true))

(event `self.ReceiveTick`
  (params (DeltaSeconds :type "Float (single-precision)"))
  (bind _widgetinteraction (`self.WidgetInteraction`))
  (bind (_returnvalue_bblockinghit _returnvalue_binitialoverlap _returnvalue_time _returnvalue_location) (`GameplayStatics.BreakHitResult` (`WidgetInteractionComponent.GetLastHitResult` _widgetinteraction)))
  ;[0 0.01484 0.11] Tick
  (`self.Check UI Interaction Status`
    (:`Is Active`
      (`SceneComponent.SetRelativeScale3D` (`self.Laser_StaticMesh`) (`KismetMathLibrary.MakeVector` (select `bool` _returnvalue_bblockinghit :`false` (`KismetMathLibrary.VSize` (- (`SceneComponent.K2_GetComponentLocation` (`self.WidgetInteraction`)) _returnvalue_location)) :`true` (`WidgetInteractionComponent.InteractionDistance` _widgetinteraction)) 0.01 0.01)))))

(event `Key|MotionController_Right_Trigger`
  (params (Key :type "Key Structure" :default "AnyKey"))
  ;[0 0.235 0.1105] Input
  (:`Pressed`
    (`self.Check UI Interaction Status`
      (:`Is Active`
        (`WidgetInteractionComponent.PressPointerKey` (`self.WidgetInteraction`) "LeftMouseButton"))))
  (:`Released`
    (`self.Check UI Interaction Status`
      (:`Is Active`
        (`WidgetInteractionComponent.ReleasePointerKey` (`self.WidgetInteraction`) "LeftMouseButton")))))

(event `Set Hit Testing Enabled`
  (params (`Is Enabled ?` :type Boolean))
  ;[0.195 0 0] Custom Events
  (set `WidgetInteractionComponent.bEnableHitTesting` `Is Enabled ?` (`self.WidgetInteraction`))
  (`SceneComponent.SetVisibility` (`self.Laser_StaticMesh`) `Is Enabled ?` false)
  (`SceneComponent.SetVisibility` (`self.BeamStart_StaticMesh`) `Is Enabled ?` false))

(fn `UserConstructionScript`)